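; BP_Restart is a trigger actor that restarts the current level when the player runs into it.
; A hit on its Trigger component by the player pawn starts a one-second camera fade, then waits two seconds.
; It then reads the current level name, starts a second one-second fade and immediately reopens that level by name.
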(event `self.Trigger.OnComponentHit`
  (params (HitComponent :type "PrimitiveComponent Object Reference") (OtherActor :type "Actor Object Reference") (OtherComp :type "PrimitiveComponent Object Reference") (NormalImpulse :type "Vector Structure") (Hit :type "HitResult Structure (by ref)"))
  (if (== OtherActor (`GameplayStatics.GetPlayerPawn` 0))
    (`PlayerCameraManager.StartCameraFade` :`self` (`GameplayStatics.GetPlayerCameraManager` 0) :`Duration` 1.0)
    (`KismetSystemLibrary.Delay` 2.0)
    (bind _returnvalue (`GameplayStatics.GetCurrentLevelName` false))
    (`PlayerCameraManager.StartCameraFade` :`self` (`GameplayStatics.GetPlayerCameraManager` 0) :`Duration` 1.0)
    (`GameplayStatics.OpenLevel` (`KismetStringLibrary.Conv_StringToName` _returnvalue) false)))

(fn `UserConstructionScript`)